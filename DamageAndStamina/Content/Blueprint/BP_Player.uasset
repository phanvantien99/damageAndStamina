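; BP_Player is the player character, handling movement, mouse look, jumping and sprinting through Enhanced Input.
; On BeginPlay it adds the IM_Control mapping context, puts the WP_Stat HUD widget on screen and refreshes it via PlayerStat.UpdateStat.
; Movement follows the control rotation, jumping only starts from the Walking mode, and sprint toggles max walk speed while held.
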(event Input|EnhancedActionEvents|EnhancedInputActionIA_LookUp
  (params (ActionValue :type Float%20%28double-precision%29) (ElapsedSeconds :type Float%20%28double-precision%29) (TriggeredSeconds :type Float%20%28double-precision%29) (InputAction :type Input%20Action%20Object%20Reference :default "/Game/Blueprint/Inputs/IA_LookUp.IA_LookUp"))
  ;[1 1 1] Mouse Control
  (:Triggered
    (Pawn|Input|AddControllerPitchInput ActionValue)))

(event Input|EnhancedActionEvents|EnhancedInputActionIA_Turn
  (params (ActionValue :type Float%20%28double-precision%29) (ElapsedSeconds :type Float%20%28double-precision%29) (TriggeredSeconds :type Float%20%28double-precision%29) (InputAction :type Input%20Action%20Object%20Reference :default "/Game/Blueprint/Inputs/IA_Turn.IA_Turn"))
  ;[1 1 1] Mouse Control
  (:Triggered
    (Pawn|Input|AddControllerYawInput ActionValue)))

(event Input|EnhancedActionEvents|EnhancedInputActionIA_MoveRight
  (params (ActionValue :type Float%20%28double-precision%29) (ElapsedSeconds :type Float%20%28double-precision%29) (TriggeredSeconds :type Float%20%28double-precision%29) (InputAction :type Input%20Action%20Object%20Reference :default "/Game/Blueprint/Inputs/IA_MoveRight.IA_MoveRight"))
  ;[1 1 1] Movement
  (:Triggered
    (Pawn|Input|AddMovementInput (Math|Vector|GetRightVector (Pawn|GetControlRotation :!class /Script/Engine.Pawn)) ActionValue false)))

(event Input|EnhancedActionEvents|EnhancedInputActionIA_Forward
  (params (ActionValue :type Float%20%28double-precision%29) (ElapsedSeconds :type Float%20%28double-precision%29) (TriggeredSeconds :type Float%20%28double-precision%29) (InputAction :type Input%20Action%20Object%20Reference :default "/Game/Blueprint/Inputs/IA_Forward.IA_Forward"))
  ;[1 1 1] Movement
  (:Triggered
    (Pawn|Input|AddMovementInput (Math|Vector|GetForwardVector (Pawn|GetControlRotation :!class /Script/Engine.Pawn)) ActionValue false)))

(event Input|EnhancedActionEvents|EnhancedInputActionIA_Sprint
  (params (ActionValue :type Boolean) (ElapsedSeconds :type Float%20%28double-precision%29) (TriggeredSeconds :type Float%20%28double-precision%29) (InputAction :type Input%20Action%20Object%20Reference :default "/Game/Blueprint/Inputs/IA_Sprint.IA_Sprint"))
  (bind _charactermovement (Variables|Character|GetCharacterMovement))
  ;[1 1 1] Sprint
  (:Triggered
    (Variables|/Script/Engine.CharacterMovementComponent|SetMaxWalkSpeed _charactermovement 7e+02))
  (:Completed
    (Variables|/Script/Engine.CharacterMovementComponent|SetMaxWalkSpeed _charactermovement 4.5e+02)))

(event Input|EnhancedActionEvents|EnhancedInputActionIA_Jump
  (params (ActionValue :type Boolean) (ElapsedSeconds :type Float%20%28double-precision%29) (TriggeredSeconds :type Float%20%28double-precision%29) (InputAction :type Input%20Action%20Object%20Reference :default "/Game/Blueprint/Inputs/IA_Jump.IA_Jump"))
  (:Triggered
    (switch Utilities|FlowControl|Switch|SwitchonEMovementMode (Variables|/Script/Engine.CharacterMovementComponent|GetMovementMode (Variables|Character|GetCharacterMovement))
      (:MOVE_Walking
        (Character|Jump))))
  (:Completed
    (Character|StopJumping)))

(event EventBeginPlay
  ;[0 0.78 1] Configuration Input
  (bind _asplayer_controller (Utilities|Casting|CastToPlayerController (Pawn|GetController)))
  (Input|AddMappingContext (PlayerController|LocalPlayerSubsystems|GetEnhancedInputLocalPlayerSubsystem _asplayer_controller) "/Game/Blueprint/Inputs/IM_Control.IM_Control" 0 "(bIgnoreAllPressedKeysUntilRelease=True,bForceImmediately=False)")
  (bind _returnvalue (UserInterface|CreateWidget "/Game/UI/WP_Stat.WP_Stat_C" (Game|GetPlayerController 0)))
  (bind _output_get (Variables|Default|SetW_HUD _returnvalue))
  (UserInterface|Viewport|AddtoViewport _output_get 0)
  (Default|UpdateStat (Variables|Default|GetPlayerStat)))

(fn ConstructionScript)