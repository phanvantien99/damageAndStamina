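; CBP_HUD is a component on BP_Player that holds health and stamina values and drives their progress bars in the player's WHUD widget.
; It caches the owning player on BeginPlay, and UpdateStat refreshes both bars from current-to-max ratios.
; Decrease functions clamp at zero and return true when depleted, while IncreaseStamina clamps at max.
; Each change pushes the new ratio to its bar through the shared UpdateWidgetFloat helper.
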(event EventBeginPlay
  (bind _asbp_player (Utilities|Casting|CastToBP_Player (Components|GetOwner)))
  (Variables|Default|SetPlayer _asbp_player))

(fn UpdateStat
  (bind _player (Variables|Default|GetPlayer))
  (bind _w_hud (Variables|/Game/Blueprint/BP_Player.BP_Player_C|GetW_HUD _player))
  (Utilities|FlowControl|Sequence
    (:then_0
      (Progress|SetPercent (Variables|/Game/UI/WP_Stat.WP_Stat_C|GetHealth _w_hud) (/ (Variables|Health|GetHealth) (Variables|Health|GetMaxHealth))))
    (:then_1
      (Progress|SetPercent (Variables|/Game/UI/WP_Stat.WP_Stat_C|GetStamina _w_hud) (/ (Variables|Stamina|GetStamina) (Variables|Stamina|GetMaxStamina))))))

(fn DecreaseHealth
  (params (HealthToDecrease :type Float%20%28double-precision%29))
  (LocalVariables|SetHealthbar (Variables|/Game/UI/WP_Stat.WP_Stat_C|GetHealth (Variables|/Game/Blueprint/BP_Player.BP_Player_C|GetW_HUD (Variables|Default|GetPlayer))))
  (if (<= (Variables|Health|GetHealth) 0.0)
    (return true)
    (elif (<= (- (Variables|Health|GetHealth) HealthToDecrease) 0.0)
      (bind _output_get (Variables|Health|SetHealth 0.0))
      (CallFunction|UpdateWidgetFloat _output_get (Variables|Health|GetMaxHealth) (LocalVariables|GetHealthbar))
      (return true)
      (else
        (bind _output_get_2 (Variables|Health|SetHealth (- (Variables|Health|GetHealth) HealthToDecrease)))
        (CallFunction|UpdateWidgetFloat _output_get_2 (Variables|Health|GetMaxHealth) (LocalVariables|GetHealthbar))
        (return false)))))

(fn UpdateWidgetFloat
  (params (CurrentValue :type Float%20%28double-precision%29) (MaxValue :type Float%20%28double-precision%29) (Bar :type Progress%20Bar%20Object%20Reference))
  (Progress|SetPercent Bar (/ CurrentValue MaxValue)))

(fn DecreaseStamina
  (params (StaminaToDecrease :type Float%20%28double-precision%29))
  (LocalVariables|SetStaminaBar (Variables|/Game/UI/WP_Stat.WP_Stat_C|GetStamina (Variables|/Game/Blueprint/BP_Player.BP_Player_C|GetW_HUD (Variables|Default|GetPlayer))))
  (if (<= (Variables|Stamina|GetStamina) 0.0)
    (return true)
    (elif (<= (- (Variables|Stamina|GetStamina) StaminaToDecrease) 0.0)
      (bind _output_get (Variables|Stamina|SetStamina 0.0))
      (CallFunction|UpdateWidgetFloat _output_get (Variables|Stamina|GetMaxStamina) (LocalVariables|GetStaminaBar))
      (return true)
      (else
        (bind _output_get_2 (Variables|Stamina|SetStamina (- (Variables|Stamina|GetStamina) StaminaToDecrease)))
        (CallFunction|UpdateWidgetFloat _output_get_2 (Variables|Stamina|GetMaxStamina) (LocalVariables|GetStaminaBar))
        (return false)))))

(fn IncreaseStamina
  (params (StaminaToIncrease :type Float%20%28double-precision%29))
  (bind _maxstamina (Variables|Stamina|GetMaxStamina))
  (LocalVariables|SetStaminaBar (Variables|/Game/UI/WP_Stat.WP_Stat_C|GetStamina (Variables|/Game/Blueprint/BP_Player.BP_Player_C|GetW_HUD (Variables|Default|GetPlayer))))
  (if (< (Variables|Stamina|GetStamina) (Variables|Stamina|GetMaxStamina))
    (if (> (+ StaminaToIncrease (Variables|Stamina|GetStamina)) (Variables|Stamina|GetMaxStamina))
      (bind _output_get (Variables|Stamina|SetStamina _maxstamina))
      (CallFunction|UpdateWidgetFloat _output_get _maxstamina (LocalVariables|GetStaminaBar))
      (else
        (bind _output_get_2 (Variables|Stamina|SetStamina (+ StaminaToIncrease (Variables|Stamina|GetStamina))))
        (CallFunction|UpdateWidgetFloat _output_get_2 (Variables|Stamina|GetMaxStamina) (LocalVariables|GetStaminaBar))))))